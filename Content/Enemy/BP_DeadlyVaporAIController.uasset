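; AI controller for the Deadly Vapor enemy that makes its pawn wander around the level.
; On possess, it starts a looping timer that fires every LoopTime.
; Each tick of the timer sends the pawn via AI MoveTo to a random reachable navigation point within MovementRadius of its current location.
; If no valid pawn is controlled, it prints a debug message instead.
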(event `self.ReceivePossess`
  (params (PossessedPawn :type "Pawn Object Reference"))
  (`KismetSystemLibrary.K2_SetTimerDelegate` (delegate `MoveToRandomLocationEvent`) (`self.LoopTime`) true))

(event `MoveToRandomLocationEvent`
  (bind _returnvalue (`self.K2_GetPawn`))
  (`/Engine/EditorBlueprintResources/StandardMacros.IsValid` _returnvalue
    (:`Is Valid`
      (`|AIMoveTo` (`self.K2_GetPawn`) (`NavigationSystemV1.K2_GetRandomReachablePointInRadius` (`self.K2_GetActorLocation` _returnvalue) (`self.MovementRadius`) null null) null))
    (:`Is Not Valid`
      (`KismetSystemLibrary.PrintText` (`|FormatText` "{0} Has no possesed pawn" (`KismetTextLibrary.Conv_StringToText` (`KismetSystemLibrary.GetDisplayName` self)))))))

(fn `UserConstructionScript`)