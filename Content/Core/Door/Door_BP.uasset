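; Door actor that blocks a passage with a forcefield, which is either up or down.
; SetDoorOpen toggles the Forcefield component's visibility and collision together: open hides it with no collision, closed shows it with query and physics collision.
; On BeginPlay it applies DefaultOpenState through the same function, with no animation or transition.
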(event `self.ReceiveBeginPlay`
  (`self.SetDoorOpen` (`self.bDefaultOpenState`)))

(fn `SetDoorOpen`
  (params (`bSet Open?` :type Boolean))
  (if `bSet Open?`
    (`SceneComponent.SetVisibility` (`self.Forcefield`) false false)
    (`PrimitiveComponent.SetCollisionEnabled` (`self.Forcefield`) "NoCollision")
    (else
      (`SceneComponent.SetVisibility` (`self.Forcefield`) true false)
      (`PrimitiveComponent.SetCollisionEnabled` (`self.Forcefield`) "QueryAndPhysics"))))

(fn `UserConstructionScript`)