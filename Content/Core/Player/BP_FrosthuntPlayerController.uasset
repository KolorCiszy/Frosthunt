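; Player controller for Frosthunt that owns the in-game HUD and manages pause, game-over and level restart.
; Each tick it feeds the PlayerState's elapsed time to the HUD timer, and pausing toggles that timer, HUD panels, cursor and input mode together.
; On the GameMode's game-ended delegate it stops the timer and records the time in the GameInstance's per-player highscore table if it is the lowest yet.
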(event `self.ReceiveBeginPlay`
  (bind _returnvalue (`|CreateWidget` "/Game/Core/UI/WBP_InGameHUD.WBP_InGameHUD_C" self))
  (bind _output_get (set `self.HUD` _returnvalue))
  (`UserWidget.AddToViewport` _output_get 0)
  (add `FrosthuntGameModeBase.GameEndedDelegate` (cast `/Game/Core/BP_FrosthuntGameModeBase` (`GameplayStatics.GetGameMode`) :!pure true) (delegate `OnGameEndedEvent`)))

(event `EnhancedInput|/Game/Core/Player/Input/IA_TogglePause`
  (params (ActionValue :type Boolean) (ElapsedSeconds :type "Float (double-precision)") (TriggeredSeconds :type "Float (double-precision)") (InputAction :type "InputAction Object Reference" :default "/Game/Core/Player/Input/IA_TogglePause.IA_TogglePause"))
  (:`Started`
    (`self.ToggleGamePaused`)))

(event `OnGameEndedEvent`
  (`self.RecieveGameEndedEvent`))

(event `OnGameRestart`
  (`WidgetBlueprintLibrary.SetInputMode_GameOnly` self true)
  (bind _returnvalue (`GameplayStatics.GetCurrentLevelName` true))
  (`GameplayStatics.OpenLevel` (`KismetStringLibrary.Conv_StringToName` _returnvalue)))

(event `self.ReceiveTick`
  (params (DeltaSeconds :type "Float (single-precision)"))
  (`/Game/Core/UI/WBP_GameTimer.UpdateTime` (`/Game/Core/UI/WBP_InGameHUD.WBP_GameTimer` (`self.HUD`)) (`FrosthuntPlayerState.GetElapsedTime` (cast `/Game/Core/Player/BP_FrosthuntPlayerState` (`self.PlayerState`) :!pure true))))

(fn `RecieveGameEndedEvent`
  (bind _asbp_frosthunt_player_state (cast `/Game/Core/Player/BP_FrosthuntPlayerState` (`self.PlayerState`) :!pure true))
  (bind _returnvalue (`PlayerState.GetPlayerName` _asbp_frosthunt_player_state))
  (bind _returnvalue_2 (`FrosthuntPlayerState.GetElapsedTime` _asbp_frosthunt_player_state))
  (bind _highscoretable (`/Game/Core/BP_GameInstance.HighscoreTable` (cast `/Game/Core/BP_GameInstance` (`GameplayStatics.GetGameInstance`) :!pure true)))
  (bind (_value _returnvalue_3) (`BlueprintMapLibrary.Map_Find` _highscoretable _returnvalue))
  (`/Game/Core/UI/WBP_InGameHUD.SetGameOverVisibility` (`self.HUD`) "Visible")
  (set `self.bShowMouseCursor` true)
  (`WidgetBlueprintLibrary.SetInputMode_GameAndUIEx` self (`self.HUD`) "DoNotLock" true true)
  (`FrosthuntPlayerState.StopGameTimer` _asbp_frosthunt_player_state)
  (`/Game/Core/UI/WBP_InGameHUD.SetCurrentScore` (`self.HUD`) _returnvalue_2)
  (if (or (< _returnvalue_2 _value) (not _returnvalue_3))
    (`BlueprintMapLibrary.Map_Add` _highscoretable _returnvalue _returnvalue_2)
    (`/Game/Core/UI/WBP_InGameHUD.SetHighScore` (`self.HUD`) _returnvalue_2)
    (else
      (`/Game/Core/UI/WBP_InGameHUD.SetHighScore` (`self.HUD`) _value))))

(fn `ToggleGamePaused`
  (bind _hud (`self.HUD`))
  (if (`GameplayStatics.IsGamePaused`)
    (`GameplayStatics.SetGamePaused` false)
    (`FrosthuntPlayerState.ResumeGameTimer` (cast `/Game/Core/Player/BP_FrosthuntPlayerState` (`self.PlayerState`) :!pure true))
    (`/Game/Core/UI/WBP_InGameHUD.SetGamePausedVisibility` (`self.HUD`) "Collapsed")
    (set `self.bShowMouseCursor` false)
    (`WidgetBlueprintLibrary.SetInputMode_GameOnly` self true)
    (else
      (`GameplayStatics.SetGamePaused` true)
      (`FrosthuntPlayerState.PauseGameTimer` (cast `/Game/Core/Player/BP_FrosthuntPlayerState` (`self.PlayerState`) :!pure true))
      (`/Game/Core/UI/WBP_InGameHUD.SetGamePausedVisibility` _hud "Visible")
      (set `self.bShowMouseCursor` true)
      (`WidgetBlueprintLibrary.SetInputMode_GameAndUIEx` self _hud "DoNotLock" true true))))

(fn `UserConstructionScript`)