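; Frosthunt game mode that spawns objective pickups and opens a random door when the objective is completed.
; On BeginPlay it binds the objective-complete and game-ended events and asks randomly chosen spawn-point actors to spawn pickups up to the objective count.
; It prints warnings for too few or invalid spawn points.
; Objective completion opens one random door of the door class, while game end only prints a message.
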(event `self.ReceiveBeginPlay`
  (add `self.GameObjCompDelegate` (delegate `OnGameObjectiveCopleteEvent`))
  (`self.SpawnPickupActors`)
  (add `self.GameEndedDelegate` (delegate `OnGameEndedEvent`)))

(event `OnGameObjectiveCopleteEvent` :!signature `self.GameObjCompDelegate`
  (params (WhoCompletedGame :type "PlayerState Object Reference"))
  (`self.UnlockRandomDoor`))

(event `OnGameEndedEvent`
  (`KismetSystemLibrary.PrintString` "game ended"))

(fn `SpawnPickupActors`
  (locals (SpawnCount :type Integer))
  (bind _pickupactorspawnclass (`self.PickupActorSpawnClass`))
  (if (`KismetSystemLibrary.IsValidClass` _pickupactorspawnclass)
    (bind _outactors (`GameplayStatics.GetAllActorsOfClass` _pickupactorspawnclass))
    (if (>= (`KismetArrayLibrary.Array_Length` _outactors) (`self.PickupItemsObjective`))
      (while (< (`local.SpawnCount`) (`self.PickupItemsObjective`))
        (bind _spawnedpickupactor (`/Game/Core/Pickup/BP_PickupActorSpawn.SpawnActor` (`KismetArrayLibrary.Array_Random` _outactors)))
        (`/Engine/EditorBlueprintResources/StandardMacros.IsValid` _spawnedpickupactor
          (:`Is Valid`
            (set `local.SpawnCount` (+ (`local.SpawnCount`) 1)))
          (:`Is Not Valid`
            (set `local.SpawnCount` (`self.PickupItemsObjective`))
            (`KismetSystemLibrary.PrintString` "There is / are invalid pickup actor spawns"))))
      (else
        (`KismetSystemLibrary.PrintString` "Too few pickup actor spawns" true true (struct :`R` 1.0 :`G` 0.006678 :`A` 1.0))))))

(fn `UnlockRandomDoor`
  (bind _outactors (`GameplayStatics.GetAllActorsOfClass` (`self.DoorClass`)))
  (`/Game/Core/Door/Door_BP.SetDoorOpen` (`KismetArrayLibrary.Array_Random` _outactors) true))

(fn `UserConstructionScript`)